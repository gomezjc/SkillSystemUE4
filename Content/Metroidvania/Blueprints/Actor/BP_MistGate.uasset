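; BP_MistGate is a gate actor that shows a notifier message when the player enters its interact collider without using mist.
; The message widget plays its intro animation with a sound cue.
; Leaving the collider, or the player's RemoveNeedMistMessage dispatcher bound on BeginPlay, plays that animation in reverse and removes the widget after a delay.
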(event `self.ReceiveBeginPlay`
  ;[1 1 1] Subscribe to remove mist message
  (`|ExecutionSequence`
    (:`then_0`
      (`parent.ReceiveBeginPlay`))
    (:`then_1`
      (add `/Game/Metroidvania/Blueprints/Characters/BP_Player.RemoveNeedMistMessage` (`self.Player`) (delegate `RemoveNeedMistMessage_Event`)))))

(event `RemoveNeedMistMessage_Event`
  ;[1 1 1] Subscribe to remove mist message
  (`self.RemoveMessage`))

(event `self.InteractCollider.OnComponentBeginOverlap`
  (params (OverlappedComponent :type "PrimitiveComponent Object Reference") (OtherActor :type "Actor Object Reference") (OtherComp :type "PrimitiveComponent Object Reference") (OtherBodyIndex :type Integer) (bFromSweep :type Boolean) (SweepResult :type "HitResult Structure (by ref)"))
  (bind _wbp_notifier (`self.WBP_Notifier`))
  ;[1 1 1] Show Message Script
  (cast `/Game/Metroidvania/Blueprints/Characters/BP_Player` OtherActor)
  (if (not (`/Game/Metroidvania/Blueprints/Characters/BP_Player.bUsingMist` (`self.Player`)))
    (set `/Game/Metroidvania/Widgets/WBP_Notify.ReceiveMessage` (`self.InteractMessage`) _wbp_notifier)
    (`UserWidget.AddToViewport` _wbp_notifier 0)
    (`UserWidget.PlayAnimation` _wbp_notifier (`/Game/Metroidvania/Widgets/WBP_Notify.Intro_NoButton` _wbp_notifier) 0.0 1 "Forward" 1.0)
    (`GameplayStatics.PlaySound2D` (`self.SFX_CanInteract`) 1.0 1.0 0.0 null null)))

(event `RemoveMessage`
  (bind _wbp_notifier (`self.WBP_Notifier`))
  (bind _intro_nobutton (`/Game/Metroidvania/Widgets/WBP_Notify.Intro_NoButton` _wbp_notifier))
  ;[1 1 1] Hide Message Script
  (`UserWidget.PlayAnimation` _wbp_notifier _intro_nobutton 0.0 1 "Reverse" 1.0 :!label _label)
  (`KismetSystemLibrary.Delay` (`WidgetAnimation.GetEndTime` _intro_nobutton))
  (`Widget.RemoveFromParent` (`self.WBP_Notifier`)))

(event `self.InteractCollider.OnComponentEndOverlap`
  (params (OverlappedComponent :type "PrimitiveComponent Object Reference") (OtherActor :type "Actor Object Reference") (OtherComp :type "PrimitiveComponent Object Reference") (OtherBodyIndex :type Integer))
  ;[1 1 1] Hide Message Script
  (cast `/Game/Metroidvania/Blueprints/Characters/BP_Player` OtherActor)
  (goto _label))

(fn `UserConstructionScript`
  (`parent.UserConstructionScript`))