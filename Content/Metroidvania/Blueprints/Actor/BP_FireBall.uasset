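; BP_FireBall is the player's fireball projectile actor, which explodes on hit and damages what it strikes.
; On Hit it spawns an impact emitter oriented by the player's current facing yaw, plays an explosion sound and shakes nearby cameras.
; It then calls DestroyActor before applying damage, reading amount and type from BP_Player's FireballAttributes.
; No movement logic appears in its graphs.
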(event `self.ReceiveHit`
  (params (MyComp :type "PrimitiveComponent Object Reference") (Other :type "Actor Object Reference") (OtherComp :type "PrimitiveComponent Object Reference") (bSelfMoved :type Boolean) (HitLocation :type "Vector Structure") (HitNormal :type "Vector Structure") (NormalImpulse :type "Vector Structure") (Hit :type "HitResult Structure (by ref)"))
  (bind _asbp_player (cast `/Game/Metroidvania/Blueprints/Characters/BP_Player` (`GameplayStatics.GetPlayerCharacter` 0)))
  (bind (_returnvalue_roll _returnvalue_pitch _returnvalue_yaw) (`KismetMathLibrary.BreakRotator` (`SceneComponent.K2_GetComponentRotation` (`Actor.RootComponent` _asbp_player))))
  (if (>= _returnvalue_yaw 0.0)
    (`GameplayStatics.SpawnEmitterAtLocation` "/Game/InfinityBladeEffects/Effects/FX_Mobile/Fire/combat/P_FireBall_Strong_MuzzFlash_01.P_FireBall_Strong_MuzzFlash_01" HitLocation (struct :`Yaw` 180.0))
    (else
      (`GameplayStatics.SpawnEmitterAtLocation` "/Game/InfinityBladeEffects/Effects/FX_Mobile/Fire/combat/P_FireBall_Strong_MuzzFlash_01.P_FireBall_Strong_MuzzFlash_01" HitLocation)))
  (`GameplayStatics.PlaySoundAtLocation` "/Game/StarterContent/Audio/Explosion_Cue.Explosion_Cue" HitLocation (struct) 1.0 1.0 0.0 null null null)
  (`GameplayStatics.PlayWorldCameraShake` "/Game/Metroidvania/Blueprints/Misc/BP_CameraShake.BP_CameraShake_C" HitLocation 0.0 1000.0)
  (`self.K2_DestroyActor`)
  (bind _asbp_player_2 (cast `/Game/Metroidvania/Blueprints/Characters/BP_Player` (`GameplayStatics.GetPlayerCharacter` 0)))
  (bind (_name _manacost _iconslate _damage _damagetype) (break `/Game/Metroidvania/Blueprints/Structs/STR_Magic_Attributes` (`/Game/Metroidvania/Blueprints/Characters/BP_Player.fireballAttributes` _asbp_player_2)))
  (`GameplayStatics.ApplyDamage` Other _damage null null _damagetype))

(fn `UserConstructionScript`)