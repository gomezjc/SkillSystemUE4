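; BP_Skill_DoubleJump is a world pickup that grants the player the double jump skill.
; Overlapping its collider enables interaction and, unless the player has the skill or is using mist, shows an animated prompt with sound.
; Interacting sets the player's skill state, plays burst effects and destroys the pickup's components.
; After a short delay for the effect, it hands a new skill-acquired widget to PC_Metroidvania to display.
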(event `self.InteractCollider.OnComponentBeginOverlap`
  (params (OverlappedComponent :type "PrimitiveComponent Object Reference") (OtherActor :type "Actor Object Reference") (OtherComp :type "PrimitiveComponent Object Reference") (OtherBodyIndex :type Integer) (bFromSweep :type Boolean) (SweepResult :type "HitResult Structure (by ref)"))
  (bind _player (`self.Player`))
  (bind _wbp_notifier (`self.WBP_Notifier`))
  ;[1 1 1] Show Interact Message
  (bind _asbp_player (cast `/Game/Metroidvania/Blueprints/Characters/BP_Player` OtherActor))
  (set `/Game/Metroidvania/Blueprints/Characters/BP_Player.BcanInteract` true _asbp_player)
  (if (`/Game/Metroidvania/Blueprints/Characters/BP_Player.bHasDoubleJump` _player)
    _
    (elif (not (`/Game/Metroidvania/Blueprints/Characters/BP_Player.bUsingMist` _player))
      (set `/Game/Metroidvania/Widgets/WBP_Notify.ReceiveMessage` (`self.InteractMessage`) _wbp_notifier)
      (`UserWidget.AddToViewport` _wbp_notifier 0)
      (`UserWidget.PlayAnimation` _wbp_notifier (`/Game/Metroidvania/Widgets/WBP_Notify.Intro` _wbp_notifier) 0.0 1 "Forward" 1.0)
      (`GameplayStatics.PlaySound2D` (`self.SFX_CanInteract`) 5.0 1.0 0.0 null null))))

(event `self.InteractCollider.OnComponentEndOverlap`
  (params (OverlappedComponent :type "PrimitiveComponent Object Reference") (OtherActor :type "Actor Object Reference") (OtherComp :type "PrimitiveComponent Object Reference") (OtherBodyIndex :type Integer))
  (bind _wbp_notifier (`self.WBP_Notifier`))
  (bind _intro (`/Game/Metroidvania/Widgets/WBP_Notify.Intro` _wbp_notifier))
  ;[1 1 1] Hide interact message script
  (cast `/Game/Metroidvania/Blueprints/Characters/BP_Player` OtherActor)
  (`UserWidget.PlayAnimation` _wbp_notifier _intro 0.0 1 "Reverse" 1.0)
  (`KismetSystemLibrary.Delay` (`WidgetAnimation.GetEndTime` _intro))
  (`Widget.RemoveFromParent` (`self.WBP_Notifier`))
  (set `/Game/Metroidvania/Blueprints/Characters/BP_Player.BcanInteract` false (`self.Player`)))

(event `/Game/Metroidvania/Blueprints/Misc/BPI_Interact.ObjectInteractivedWith`
  (bind _player (`self.Player`))
  ;[1 1 1] Player acquired double jump
  (if (`/Game/Metroidvania/Blueprints/Characters/BP_Player.bHasDoubleJump` _player)
    (`KismetSystemLibrary.PrintString` "has double jump")
    (else
      (set `/Game/Metroidvania/Blueprints/Characters/BP_Player.bHasDoubleJump` true _player)
      (set `/Game/Metroidvania/Blueprints/Characters/BP_Player.SkillAcquired` "NewEnumerator1" _player)
      (`self.playerAcquiredSkillFX`)
      (`KismetSystemLibrary.Delay` 0.7) ; Para que termine la animacion FX
      (bind _returnvalue (`|CreateWidget` "/Game/Metroidvania/Widgets/WBP_SkillAcquired.WBP_SkillAcquired_C"))
      (bind _aspc_metroidvania (cast `/Game/Metroidvania/Framework/PC_MetroidVania` (`GameplayStatics.GetPlayerController` 0)))
      (set `/Game/Metroidvania/Framework/PC_MetroidVania.WPB_LearnSkill` _returnvalue _aspc_metroidvania)
      (`/Game/Metroidvania/Framework/PC_MetroidVania.ShowAcquiredSkill` _aspc_metroidvania))))

(fn `playerAcquiredSkillFX`
  (`Widget.RemoveFromParent` (`self.WBP_Notifier`))
  (`GameplayStatics.SpawnEmitterAtLocation` "/Game/InfinityBladeEffects/Effects/FX_Treasure/Resources/P_OrePile_Explosion_Success.P_OrePile_Explosion_Success" (`SceneComponent.K2_GetComponentLocation` (`self.SkillMesh`)) (struct) (2.0 2.0 2.0))
  (`GameplayStatics.PlaySound2D` "/Game/Metroidvania/Audio/SFX_SkillAcquired.SFX_SkillAcquired" 3.0 1.0 0.0 null null)
  (`ActorComponent.K2_DestroyComponent` (`self.SkillMesh`))
  (`ActorComponent.K2_DestroyComponent` (`self.SkillVFX`))
  (`ActorComponent.K2_DestroyComponent` (`self.SkillLight`))
  (`ActorComponent.K2_DestroyComponent` (`self.InteractCollider`)))

(fn `UserConstructionScript`
  (`parent.UserConstructionScript`))