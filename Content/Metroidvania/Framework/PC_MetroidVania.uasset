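; Player controller for the Metroidvania game that runs the black and white magic menus and the acquired-skill popup.
; Holding a magic input swaps the HUD for its menu, created at BeginPlay, and pauses; release restores play and animates the HUD slot if a selection was made.
; White magic release passes through a gate opened on press; its readiness check is hardwired true.
; The skill popup pauses until dismissed by input.
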(event `self.ReceiveBeginPlay`
  (`|ExecutionSequence`
    (:`then_0`
      ;[1 1 1] BMagic Menu Reference
      (bind _returnvalue (`|CreateWidget` "/Game/Metroidvania/Widgets/WBP_BMagic_Menu.WBP_BMagic_Menu_C"))
      (set `self.WBP_Bmagic_Menu` _returnvalue))
    (:`then_1`
      ;[1 1 1] WMagic Menu Reference
      (bind _returnvalue_2 (`|CreateWidget` "/Game/Metroidvania/Widgets/WBP_WMagic_Menu.WBP_WMagic_Menu_C"))
      (set `self.WBP_Wmagic_Menu` _returnvalue_2))))

(event `InputAction|BlackMagicMenu` :paused true
  (params (Key :type "Key Structure"))
  (bind _returnvalue (`GameplayStatics.GetPlayerController` 0))
  (bind _wbp_bmagic_menu (`self.WBP_Bmagic_Menu`))
  ;[1 1 1] Show/Hide Black Magic Menu
  (:`Pressed`
    (bind _asmv_hud (cast `/Game/Metroidvania/Framework/MV_HUD` (`self.GetHUD`)))
    (bind _wbp_hud (`/Game/Metroidvania/Framework/MV_HUD.WBP_HUD` _asmv_hud))
    (`Widget.RemoveFromParent` _wbp_hud)
    (`UserWidget.AddToViewport` _wbp_bmagic_menu 0)
    (`UserWidget.PlayAnimation` _wbp_bmagic_menu (`/Game/Metroidvania/Widgets/WBP_BMagic_Menu.BMagicMenuIntro` _wbp_bmagic_menu) 0.0 1 "Forward" 1.0)
    (`GameplayStatics.PlaySound2D` (`self.SFX_Menu_On`) 1.0 1.0 0.0 null null)
    (`GameplayStatics.SetGamePaused` true)
    (`WidgetBlueprintLibrary.SetInputMode_GameAndUIEx` _returnvalue (`self.WBP_Bmagic_Menu`)))
  (:`Released`
    (`UserWidget.AddToViewport` _wbp_hud 0)
    (`Widget.RemoveFromParent` _wbp_bmagic_menu)
    (`GameplayStatics.PlaySound2D` (`self.SFX_Menu_Off`) 1.0 1.0 0.0 null null)
    (`GameplayStatics.SetGamePaused` false)
    (`WidgetBlueprintLibrary.SetInputMode_GameOnly` _returnvalue)
    ;[1 1 1] ShowStartbust Upon Selection
    (if (`/Game/Metroidvania/Widgets/WBP_BMagic_Menu.bSelectionMade` (`self.WBP_Bmagic_Menu`))
      (`GameplayStatics.PlaySound2D` (`self.SFX_Magic_Slotted`) 1.0 1.0 0.0 null null)
      (bind _asmv_hud_2 (cast `/Game/Metroidvania/Framework/MV_HUD` (`self.GetHUD`)))
      (bind _wbp_hud_2 (`/Game/Metroidvania/Framework/MV_HUD.WBP_HUD` _asmv_hud_2))
      (`UserWidget.PlayAnimation` _wbp_hud_2 (`/Game/Metroidvania/Widgets/WBP_HUD.BMagicSlotted` _wbp_hud_2) 0.0 1 "Forward" 1.0))))

(event `InputAction|WhiteMagicMenu` :paused true
  (params (Key :type "Key Structure"))
  (bind _returnvalue (`GameplayStatics.GetPlayerController` 0))
  (bind _wbp_wmagic_menu (`self.WBP_Wmagic_Menu`))
  ;[1 1 1] Show/Hide White Magic Menu
  (:`Pressed`
    (bind _asbp_player (cast `/Game/Metroidvania/Blueprints/Characters/BP_Player` (`GameplayStatics.GetPlayerCharacter` 0)))
    (if true
      (`|ExecutionSequence`
        (:`then_0`
          (bind _asmv_hud (cast `/Game/Metroidvania/Framework/MV_HUD` (`self.GetHUD`)))
          (bind _wbp_hud (`/Game/Metroidvania/Framework/MV_HUD.WBP_HUD` _asmv_hud))
          (`Widget.RemoveFromParent` _wbp_hud)
          (`UserWidget.AddToViewport` _wbp_wmagic_menu 0)
          (`UserWidget.PlayAnimation` _wbp_wmagic_menu (`/Game/Metroidvania/Widgets/WBP_WMagic_Menu.WMagicMenuIntro` _wbp_wmagic_menu) 0.0 1 "Forward" 1.0)
          (`GameplayStatics.PlaySound2D` (`self.SFX_Menu_On`) 1.0 1.0 0.0 null null)
          (`GameplayStatics.SetGamePaused` true)
          (`WidgetBlueprintLibrary.SetInputMode_GameAndUIEx` _returnvalue (`self.WBP_Wmagic_Menu`)))
        (:`then_1`
          (goto _label :!via `Open`)))
      (else
        (`GameplayStatics.PlaySound2D` (`self.SFX_Action_Disallowed`) 0.3 1.0 0.0 null null))))
  (:`Released`
    (`/Engine/EditorBlueprintResources/StandardMacros.Gate` true :!label _label
      (:`Exit`
        (`|ExecutionSequence`
          (:`then_0`
            (`UserWidget.AddToViewport` _wbp_hud 0)
            (`Widget.RemoveFromParent` _wbp_wmagic_menu)
            (`GameplayStatics.PlaySound2D` (`self.SFX_Menu_Off`) 1.0 1.0 0.0 null null)
            (`GameplayStatics.SetGamePaused` false)
            (`WidgetBlueprintLibrary.SetInputMode_GameOnly` _returnvalue)
            ;[1 1 1] ShowStartbust Upon Selection
            (if (`/Game/Metroidvania/Widgets/WBP_WMagic_Menu.bSelectionMade` (`self.WBP_Wmagic_Menu`))
              (`GameplayStatics.PlaySound2D` (`self.SFX_Magic_Slotted`) 1.0 1.0 0.0 null null)
              (bind _asmv_hud_2 (cast `/Game/Metroidvania/Framework/MV_HUD` (`self.GetHUD`)))
              (bind _wbp_hud_2 (`/Game/Metroidvania/Framework/MV_HUD.WBP_HUD` _asmv_hud_2))
              (`UserWidget.PlayAnimation` _wbp_hud_2 (`/Game/Metroidvania/Widgets/WBP_HUD.WMagicSlotted` _wbp_hud_2) 0.0 1 "Forward" 1.0)))
          (:`then_1`
            (goto _label :!via `Close`)))))))

(event `ShowAcquiredSkill`
  ;[1 1 1] Show acquired skill
  (`GameplayStatics.SetGamePaused` true)
  (`UserWidget.AddToViewport` (`self.WPB_LearnSkill`) 0))

(event `InputAction|ExitSkillAcquired` :consume false :paused true
  (params (Key :type "Key Structure"))
  (bind _returnvalue (`GameplayStatics.GetPlayerController` 0))
  (bind _wpb_learnskill (`self.WPB_LearnSkill`))
  ;[1 1 1] Hide acquired skill widget blueprint
  (:`Pressed`
    (if (`GameplayStatics.IsGamePaused`)
      (`/Engine/EditorBlueprintResources/StandardMacros.IsValid` _wpb_learnskill
        (:`Is Valid`
          (`Widget.RemoveFromParent` _wpb_learnskill)
          (`GameplayStatics.SetGamePaused` false)
          (`WidgetBlueprintLibrary.SetInputMode_GameOnly` _returnvalue)
          (set `PlayerController.bShowMouseCursor` false _returnvalue))))))

(fn `UserConstructionScript`)